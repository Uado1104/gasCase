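; BP_Player1 is a player character Blueprint whose one custom function, LockCamera, switches between a locked and a free camera.
; When locked, the character takes controller yaw, the spring arm ignores control rotation, and the camera is raised and pitched down.
; When unlocked, the spring arm follows control rotation, the character orients to movement, and the camera's relative transform resets.
; The event graph holds only disabled stub events.
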(fn `LockCamera`
  (params (IsLock :type Boolean))
  (bind _springarm (`self.SpringArm`))
  (bind _charactermovement (`self.CharacterMovement`))
  (bind _camera (`self.Camera`))
  (if IsLock
    (set `self.bUseControllerRotationYaw` true)
    (set `SpringArmComponent.bUsePawnControlRotation` false _springarm)
    (set `CharacterMovementComponent.bOrientRotationToMovement` false _charactermovement)
    (`SceneComponent.K2_SetRelativeLocationAndRotation` _camera (0.0 0.0 200.0) (struct :`Pitch` -20.0) false false)
    (else
      (set `self.bUseControllerRotationYaw` false)
      (set `SpringArmComponent.bUsePawnControlRotation` true _springarm)
      (set `CharacterMovementComponent.bOrientRotationToMovement` true _charactermovement)
      (`SceneComponent.K2_SetRelativeLocationAndRotation` :`self` _camera))))

(fn `UserConstructionScript`
  (`parent.UserConstructionScript`))
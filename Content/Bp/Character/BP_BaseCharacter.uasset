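; BP_BaseCharacter is a character Blueprint that uses the Gameplay Ability System for melee.
; BeginPlay grants GAS_Melee, and the Melee event calls ActivateAbility with index 0, which tries to activate abilities by the tag container stored at that index.
; A capsule overlap handler filters the other actor by class and against self, casts it to BaseCharacter and prints its display name.
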(event `self.ReceiveBeginPlay`
  (`AbilitySystemComponent.K2_GiveAbility` (`self.AbilitySystem`) "/Game/Bp/Ability/00Melee/GAS_Melee.GAS_Melee_C" 0 -1))

(event `Melee`
  (`self.ActivateAbility` 0))

(event `self.Capsule.OnComponentBeginOverlap`
  (params (OverlappedComponent :type "PrimitiveComponent Object Reference") (OtherActor :type "Actor Object Reference") (OtherComp :type "PrimitiveComponent Object Reference") (OtherBodyIndex :type Integer) (bFromSweep :type Boolean) (SweepResult :type "HitResult Structure (by ref)"))
  (if (and (!= (`GameplayStatics.GetObjectClass` OtherActor) null) (!= OtherActor self))
    (bind _asbase_character (cast `BaseCharacter` OtherActor))
    (`KismetSystemLibrary.PrintString` (`KismetSystemLibrary.GetDisplayName` _asbase_character))))

(fn `ActivateAbility`
  (params (AbilityIdnex :type Integer))
  (`AbilitySystemComponent.TryActivateAbilitiesByTag` (`self.AbilitySystem`) (`|GetArrayItem` (`self.Gameplay Tag Container`) AbilityIdnex) true))

(fn `UserConstructionScript`)